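; Base actor for a targetable, damageable ship component that the player ship can lock as a weapons target.
; Highlight toggles custom depth on the mesh and all its children, likely for outline rendering.
; TakeDamage clamps health and fires Death once at zero, clearing highlight and the player's target.
; Death then either spawns an effect and destroys the actor, or attaches the effect and disables collision, per DestroyOnDeath.
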(event Custom|Highlight
  (params (Active :type Boolean))
  (bind _mesh (Variables|Default|GetMesh))
  (bind _mesh_2 (Variables|Default|GetMesh))
  (if Active
    (Rendering|SetRenderCustomDepth _mesh_2 true)
    (for _array_element (Components|GetChildrenComponents _mesh_2 true)
      (bind _asprimitive_component (Utilities|Casting|CastToPrimitiveComponent _array_element))
      (Rendering|SetRenderCustomDepth _asprimitive_component true))
    (else
      (Rendering|SetRenderCustomDepth _mesh false)
      (for _array_element_2 (Components|GetChildrenComponents _mesh true)
        (bind _asprimitive_component_2 (Utilities|Casting|CastToPrimitiveComponent _array_element_2))
        (Rendering|SetRenderCustomDepth _asprimitive_component_2 false)))))

(event Custom|TakeDamage
  (params (Damage :type Float%20%28single-precision%29))
  (bind _output_get (Variables|Default|SetHealth (Math|Float|Clamp(Float) (- (Variables|Default|GetHealth) Damage) 0.0 (Variables|Default|GetMaxHealth))))
  (if (== _output_get 0.0)
    (Utilities|FlowControl|DoOnce false
      (:Completed
        (CallFunction|Death)))))

(event Custom|Death
  (bind _returnvalue (Transformation|GetActorTransform))
  (bind _deatheffect (Variables|Default|GetDeathEffect))
  (CallFunction|Highlight false)
  (bind _asbp_player_ship (Utilities|Casting|CastToBP_PlayerShip (Game|Player|GetPlayerPawn 0)))
  (if (== (Variables|/Game/Blueprints/BP_PlayerShip.BP_PlayerShip_C|GetWeaponsTarget _asbp_player_ship) self)
    (Variables|/Game/Blueprints/BP_PlayerShip.BP_PlayerShip_C|SetWeaponsTarget _asbp_player_ship 0))
  (if (Variables|Default|GetDestroyOnDeath)
    (Effects|SpawnEmitteratLocation _deatheffect (.location _returnvalue) (.rotation _returnvalue))
    (Utilities|FlowControl|Delay 0.08)
    (Actor|DestroyActor)
    (else
      (Effects|SpawnEmitterAttached _deatheffect (Variables|Default|GetMesh) "None" (.location _returnvalue) (.rotation _returnvalue) "1.000000,1.000000,1.000000" "KeepWorldPosition")
      (Collision|SetCollisionEnabled (Variables|Default|GetMesh) "NoCollision")
      (for _array_element (Components|GetChildrenComponents (Variables|Default|GetMesh) true)
        (bind _asprimitive_component (Utilities|Casting|CastToPrimitiveComponent _array_element))
        (Collision|SetCollisionEnabled _asprimitive_component "NoCollision")))))

(fn ConstructionScript)

(fn Init)