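; Player ship that rides the BP_SlipspaceTube spline in a rhythm-driven shooter.
; A looping timer moves ShipCenter along the track, eases 30-degree lane rolls and hover distance, and scales FOV with speed.
; Thrust presses are graded by MusicManager beat closeness, adjusting speed, damage bonus and HUD streak; Perfect hits delay slowdown.
; It also fires child-actor turrets by slot and handles cockpit and reverse cameras.
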(event Custom|Init
  ;[1 1 1] Init
  (CallFunction|InitHelpers)
  (Utilities|Time|SetTimerbyEvent (delegate Custom|Update) 0.005 true)
  (bind _returnvalue (UserInterface|CreateWidget "/Game/Blueprints/Widget_PlayerHUD.Widget_PlayerHUD_C" 0 self (Variables|Default|GetMusicManager)))
  (bind _output_get (Variables|Default|SetHUD _returnvalue))
  (UserInterface|Viewport|AddtoViewport _output_get 0)
  (CallFunction|InitWeapons))

(event Custom|Update
  (bind _shipcenter (Variables|Default|GetshipCenter))
  (bind _shipcenter_2 (Variables|Default|GetshipCenter))
  (bind _slipspacetrack (Variables|Default|GetSlipspaceTrack))
  (bind _returnvalue (Transformation|GetWorldRotation _shipcenter_2))
  (bind _spline (Variables|/Game/Blueprints/BP_SlipspaceTube.BP_SlipspaceTube_C|GetSpline _slipspacetrack))
  (bind _relativerotation (Variables|/Script/Engine.SceneComponent|GetRelativeRotation _shipcenter))
  (bind (_roll _pitch _yaw) (Math|Rotator|BreakRotator _relativerotation))
  (bind (_roll_2 _pitch_2) (Math|Rotator|BreakRotator _returnvalue))
  (Utilities|FlowControl|Sequence
    (:then_0
      ;[1 1 1] Update ship location along spline
      (bind _output_get (Variables|ShipMovement|SettrackDist (+ (Variables|ShipMovement|GettrackDist) (* (Variables|ShipMovement|GetLinearVelocity) (Variables|ShipMovement|GetSpeedBoost)))))
      (Transformation|SetWorldLocation _shipcenter_2 (Spline|GetLocationatDistanceAlongSpline _spline (Math|Float|%(Float) _output_get (Spline|GetSplineLength _spline)) "World") false false)
      (Transformation|SetWorldRotation _shipcenter_2 (Math|Rotator|Lerp(Rotator) _returnvalue (Math|Rotator|MakeRotator _roll_2 _pitch_2 (.yaw (Spline|GetRotationatDistanceAlongSpline _spline (Math|Float|%(Float) _output_get (Spline|GetSplineLength _spline)) "World"))) 0.08 true) false false)
      ;[1 1 1] lerp 30 degree strafing (unused)
      (Transformation|SetRelativeRotation _shipcenter (Math|Rotator|Lerp(Rotator) _relativerotation (Math|Rotator|MakeRotator (Variables|ShipMovement|GettargetLaneDegree) _pitch _yaw) 0.03 true) false false)
      ;[1 1 1] Update ship rotation and hover dist
      (bind _output_get_2 (Variables|ShipMovement|SethoverDist (Math|Float|Lerp (Variables|ShipMovement|GethoverDist) (Variables|ShipMovement|GettargetHoverDist) 0.03)))
      (Transformation|SetRelativeLocation (Variables|Default|GetStaticMesh) (Math|Vector|MakeVector 0.0 0.0 _output_get_2) false false))
    (:then_1
      ;[1 1 1] Slow down
      (if (Variables|ShipMovement|GetisSlowingDown)
        (Variables|ShipMovement|SetLinearVelocity (Math|Float|Lerp (Variables|ShipMovement|GetLinearVelocity) (Variables|ShipMovement|GetMinLinearVelocity) 0.003))
        (Variables|ShipMovement|SetTargetLinearVelocity (Math|Float|Lerp (Variables|ShipMovement|GetLinearVelocity) (Variables|ShipMovement|GetMinLinearVelocity) 0.003))
        (else
          (Variables|ShipMovement|SetLinearVelocity (Math|Float|Lerp (Variables|ShipMovement|GetLinearVelocity) (Variables|ShipMovement|GetTargetLinearVelocity) 0.01))))
      (Camera|SetFieldOfView (Variables|Default|GetMainCamera) (+ (- 9e+01 (Variables|ShipMovement|GetMinLinearVelocity)) (* (Variables|ShipMovement|GetLinearVelocity) 0.5))))))

(event Custom|StartSlowingDown
  ;[1 1 1] Add linear thrust
  (Variables|ShipMovement|SetisSlowingDown true)
  (Development|PrintString "SlowingDown!"))

(event EventBeginPlay
  ;[1 1 1] Init
  (CallFunction|Init)
  (bind _outactors (Actor|GetAllActorsOfClass "/Game/Blueprints/BP_SlipspaceTube.BP_SlipspaceTube_C"))
  (Variables|Default|SetSlipspaceTrack (Utilities|Array|Get(acopy) _outactors))
  (Variables|ShipMovement|SetTargetLinearVelocity (Variables|ShipMovement|GetMinLinearVelocity)))

(event Input|ActionEvents|InputActionChangeCamera
  (params (Key :type Key%20Structure))
  (bind _cockpitcamera (Variables|Default|GetCockpitCamera))
  (bind _maincamera (Variables|Default|GetMainCamera))
  ;[1 1 1] Camera Controls
  (:Pressed
    (if (Variables|Default|GetisFirstPerson)
      (Components|Activation|SetActive _maincamera true false)
      (Components|Activation|SetActive _cockpitcamera false false)
      (Variables|Default|SetisFirstPerson false)
      (else
        (Components|Activation|SetActive _maincamera false false)
        (Components|Activation|SetActive _cockpitcamera true false)
        (Variables|Default|SetisFirstPerson true)))))

(event Input|ActionEvents|InputActionAddThrust
  (params (Key :type Key%20Structure))
  (bind _minlinearvelocity (Variables|ShipMovement|GetMinLinearVelocity))
  (bind _hud (Variables|Default|GetHUD))
  (bind _hud_2 (Variables|Default|GetHUD))
  (bind _maxlinearvelocity (Variables|ShipMovement|GetMaxLinearVelocity))
  ;[1 1 1] Add linear thrust
  (:Pressed
    (if (< (Variables|ShipMovement|GetLinearVelocity) (- (Variables|ShipMovement|GetMaxLinearVelocity) 0.1))
      (bind _closeness (Default|GetonBeatCloseness (Variables|Default|GetMusicManager)))
      (Default|UpdateonBeatText (Variables|Default|GetHUD) _closeness)
      (switch Utilities|FlowControl|Switch|SwitchonOnBeat _closeness
        (:NewEnumerator0
          (Variables|ShipMovement|SetTargetLinearVelocity (Math|Float|Clamp(Float) (+ (Variables|ShipMovement|GetTargetLinearVelocity) 5.0) _minlinearvelocity _maxlinearvelocity))
          (Variables|Combat|SetWeaponDmgBonus (Math|Float|Clamp(Float) (+ (Variables|Combat|GetWeaponDmgBonus) 0.1) 0.0 (Variables|Combat|GetMaxWeaponDmgBonus)))
          (if (> (Variables|/Game/Blueprints/Widget_PlayerHUD.Widget_PlayerHUD_C|GetSyncNum _hud) 0)
            (Default|IncStreak _hud)
            (else
              (Default|BeginStreak _hud)))
          (Utilities|Time|SetTimerbyEvent (delegate Custom|StartSlowingDown) (Variables|ShipMovement|GetSlowdownCooldown))
          (Variables|ShipMovement|SetisSlowingDown false))
        (:NewEnumerator1
          (Variables|ShipMovement|SetTargetLinearVelocity (Math|Float|Clamp(Float) (+ (Variables|ShipMovement|GetTargetLinearVelocity) 3.0) _minlinearvelocity _maxlinearvelocity))
          (Variables|Combat|SetWeaponDmgBonus (Math|Float|Clamp(Float) (+ (Variables|Combat|GetWeaponDmgBonus) 0.02) 0.0 (Variables|Combat|GetMaxWeaponDmgBonus)))
          (if (> (Variables|/Game/Blueprints/Widget_PlayerHUD.Widget_PlayerHUD_C|GetSyncNum _hud_2) 0) :!label _label
            (Default|StreakBroken _hud_2)))
        (:NewEnumerator2
          (Variables|ShipMovement|SetTargetLinearVelocity (Math|Float|Clamp(Float) (+ (Variables|ShipMovement|GetTargetLinearVelocity) 2.0) _minlinearvelocity _maxlinearvelocity))
          (goto _label))
        (:NewEnumerator3
          (Variables|ShipMovement|SetTargetLinearVelocity (Math|Float|Clamp(Float) (+ (Variables|ShipMovement|GetTargetLinearVelocity) -2.0) _minlinearvelocity _maxlinearvelocity))
          (goto _label))))))

(event Input|ActionEvents|InputActionAddStrafe_Left
  (params (Key :type Key%20Structure))
  ;[1 1 1] 30 degree strafe
  (:Pressed
    (Variables|ShipMovement|SettargetLaneDegree (+ (Variables|ShipMovement|GettargetLaneDegree) 3e+01))))

(event Input|ActionEvents|InputActionAddStrafe_Right
  (params (Key :type Key%20Structure))
  ;[1 1 1] 30 degree strafe
  (:Pressed
    (Variables|ShipMovement|SettargetLaneDegree (+ (Variables|ShipMovement|GettargetLaneDegree) -3e+01))))

(event Input|ActionEvents|InputActionReverseCamera
  (params (Key :type Key%20Structure))
  (bind _springarm (Variables|Default|GetSpringArm))
  (bind _cockpitcamera (Variables|Default|GetCockpitCamera))
  ;[1 1 1] Camera Controls
  (:Pressed
    (bind _output_get (Variables|Default|SetReversedCamera (not (Variables|Default|GetReversedCamera)) :!label _label))
    (if _output_get
      (Transformation|SetRelativeRotation _springarm "0,180.000000, 0" false false)
      (Transformation|SetRelativeLocation _cockpitcamera "0, 0,150.000000" false false)
      (else
        (Transformation|SetRelativeRotation _springarm "0, 0, 0" false false)
        (Transformation|SetRelativeLocation _cockpitcamera "0, 0,150.000000" false false))))
  (:Released
    (goto _label)))

(event Input|ActionEvents|InputActionFire_Weapon2
  (params (Key :type Key%20Structure))
  (:Pressed
    (for _array_element (Variables|Default|GetWeapons)
      (if (and (Variables|/Game/Blueprints/PlayerWeapons/BP_PlayerTurret.BP_PlayerTurret_C|GetCanFire _array_element) (== (Variables|/Game/Blueprints/PlayerWeapons/BP_PlayerTurret.BP_PlayerTurret_C|GetSlot _array_element) 1))
        (Default|Fire _array_element))))
  (:Released
    (for _array_element_2 (Variables|Default|GetWeapons)
      (if (== (Variables|/Game/Blueprints/PlayerWeapons/BP_PlayerTurret.BP_PlayerTurret_C|GetSlot _array_element_2) 1)
        (Default|StopFiring _array_element_2)))))

(event Input|ActionEvents|InputActionFire_Weapon1
  (params (Key :type Key%20Structure))
  (:Pressed
    (for _array_element (Variables|Default|GetWeapons)
      (if (and (Variables|/Game/Blueprints/PlayerWeapons/BP_PlayerTurret.BP_PlayerTurret_C|GetCanFire _array_element) (== (Variables|/Game/Blueprints/PlayerWeapons/BP_PlayerTurret.BP_PlayerTurret_C|GetSlot _array_element) 0))
        (Default|Fire _array_element))))
  (:Released
    (for _array_element_2 (Variables|Default|GetWeapons)
      (if (== (Variables|/Game/Blueprints/PlayerWeapons/BP_PlayerTurret.BP_PlayerTurret_C|GetSlot _array_element_2) 0)
        (Default|StopFiring _array_element_2)))))

(event Input|AxisEvents|InputAxisWheelDist
  (params (AxisValue :type Float%20%28single-precision%29))
  ;[1 1 1] Hover Dist
  (if (!= AxisValue 0.0)
    (Variables|ShipMovement|SettargetHoverDist (Math|Float|Clamp(Float) (+ (Variables|ShipMovement|GettargetHoverDist) (* AxisValue 125.0)) -1.4e+03 -4e+02))))

(event Input|AxisEvents|InputAxisThrust
  (params (AxisValue :type Float%20%28single-precision%29))
  ;[1 1 1] Add linear braking
  (if (< AxisValue 0.0)
    (Variables|ShipMovement|SetTargetLinearVelocity (Math|Float|Clamp(Float) (+ (Variables|ShipMovement|GetTargetLinearVelocity) (* (Variables|ShipMovement|GetDecceleration) AxisValue)) 0.0 (Variables|ShipMovement|GetMaxLinearVelocity)))))

(event Input|AxisEvents|InputAxisStrafe
  (params (AxisValue :type Float%20%28single-precision%29))
  (bind _maxstrafevelocity (Variables|ShipMovement|GetMaxStrafeVelocity))
  ;[1 1 1] Smooth strafe
  (if (!= AxisValue 0.0)
    (Variables|ShipMovement|SetstrafeVelocity (Math|Float|Clamp(Float) (+ (Variables|ShipMovement|GetstrafeVelocity) (* (Variables|ShipMovement|GetStrafeAcceleration) AxisValue)) (* _maxstrafevelocity -1.0) _maxstrafevelocity))
    (else
      (Variables|ShipMovement|SetstrafeVelocity (Math|Float|Lerp (Variables|ShipMovement|GetstrafeVelocity) 0.0 0.01)))))

(fn ConstructionScript)

(fn InitWeapons
  (for _array_element (Actor|GetAllChildActors true)
    (bind _asbp_player_turret (Utilities|Casting|CastToBP_PlayerTurret _array_element))
    (Variables|/Game/Blueprints/PlayerWeapons/BP_PlayerTurret.BP_PlayerTurret_C|SetPlayer _asbp_player_turret self)
    (Default|Init _asbp_player_turret)
    (Utilities|Array|Add (Variables|Default|GetWeapons) _asbp_player_turret))
  (bind _outactors (Actor|GetAllActorsOfClass "/Game/Blueprints/BP_EnemyShip.BP_EnemyShip_C"))
  (Variables|Default|SetEnemyShip (Utilities|Array|Get(acopy) _outactors)))

(fn InitHelpers
  (bind _outactors (Actor|GetAllActorsOfClass "/Game/Blueprints/BP_MusicManager.BP_MusicManager_C"))
  (Variables|Default|SetMusicManager (Utilities|Array|Get(acopy) _outactors))
  (Variables|/Script/Engine.PlayerController|SetbShowMouseCursor (Game|GetPlayerController 0) true))