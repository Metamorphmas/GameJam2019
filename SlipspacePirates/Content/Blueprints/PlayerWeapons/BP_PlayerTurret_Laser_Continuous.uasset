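; Continuous laser player turret that deals repeated damage to the player's weapons target while draining the player's weapon damage bonus as energy.
; Fire shows a beam plane stretched to the target distance variable and starts a looping damage timer.
; Each tick damages a valid, visible target, drains energy regardless, and stops firing when energy runs low.
; Construction gives the beam a dynamic material instance.
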(event Custom|DealDamage
  (bind _player (Variables|Default|GetPlayer))
  (bind _energydrain (Variables|Default|GetEnergyDrain))
  (if (and (Utilities|IsValid (Variables|/Game/Blueprints/BP_PlayerShip.BP_PlayerShip_C|GetWeaponsTarget (Variables|Default|GetPlayer))) (Variables|Default|GetCanSee))
    (Default|TakeDamage (Variables|/Game/Blueprints/BP_PlayerShip.BP_PlayerShip_C|GetWeaponsTarget (Variables|Default|GetPlayer)) (Variables|Default|GetDamage)))
  (bind _output_get (Variables|/Game/Blueprints/BP_PlayerShip.BP_PlayerShip_C|SetWeaponDmgBonus _player (Math|Float|Clamp(Float) (- (Variables|/Game/Blueprints/BP_PlayerShip.BP_PlayerShip_C|GetWeaponDmgBonus _player) _energydrain) 0.0 (Variables|/Game/Blueprints/BP_PlayerShip.BP_PlayerShip_C|GetMaxWeaponDmgBonus _player))))
  (if (< _output_get _energydrain)
    (CallFunction|StopFiring)))

(event EventFire
  (bind _laserplane (Variables|Default|GetLaserPlane))
  (if (>= (Variables|/Game/Blueprints/BP_PlayerShip.BP_PlayerShip_C|GetWeaponDmgBonus (Variables|Default|GetPlayer)) (Variables|Default|GetEnergyDrain))
    (Variables|Default|SetCanFire false)
    (Development|SetHiddeninGame _laserplane false false)
    (Transformation|SetRelativeScale3D _laserplane (Math|Vector|MakeVector (Variables|Default|GetDist) 2.0 2.0))
    (bind _returnvalue (Utilities|Time|SetTimerbyEvent (delegate Custom|DealDamage) 0.1 true))))

(event EventStopFiring
  (Development|SetHiddeninGame (Variables|Default|GetLaserPlane) true false)
  (Variables|Default|SetCanFire true)
  (Utilities|Time|ClearandInvalidateTimerbyHandle (stale EventFire _returnvalue)))

(fn ConstructionScript
  (bind _returnvalue (Rendering|Material|CreateDynamicMaterialInstance "/Game/Materials/MI_Laser_2.MI_Laser_2" "None" :!class /Script/Engine.KismetMaterialLibrary))
  (bind _output_get (Variables|Default|SetLaserMat _returnvalue))
  (Rendering|Material|SetMaterial (Variables|Default|GetLaserPlane) 0 _output_get))