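; BP_PlayerTurret_Laser is a player turret that fires a laser at the player's current weapons target.
; Fire spends EnergyDrain from the player's WeaponDmgBonus pool, then shows a plane stretched to the target distance.
; A timeline drives the glow of its dynamic lightning material, then hides the plane and re-enables firing.
; Damage applies instantly, only if the target is valid and visible.
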(event EventFire
  (bind _laserplane (Variables|Default|GetLaserPlane))
  (bind _player (Variables|Default|GetPlayer))
  (bind _energydrain (Variables|Default|GetEnergyDrain))
  (if (>= (Variables|/Game/Blueprints/BP_PlayerShip.BP_PlayerShip_C|GetWeaponDmgBonus _player) _energydrain)
    (Variables|Default|SetCanFire false)
    (Variables|/Game/Blueprints/BP_PlayerShip.BP_PlayerShip_C|SetWeaponDmgBonus _player (Math|Float|Clamp(Float) (- (Variables|/Game/Blueprints/BP_PlayerShip.BP_PlayerShip_C|GetWeaponDmgBonus _player) _energydrain) 0.0 (Variables|/Game/Blueprints/BP_PlayerShip.BP_PlayerShip_C|GetMaxWeaponDmgBonus _player)))
    (Development|SetHiddeninGame _laserplane false false)
    (Transformation|SetRelativeScale3D _laserplane (Math|Vector|MakeVector (Variables|Default|GetDist) 2.0 2.0))
    (Utilities|FlowControl|Sequence
      (:then_0
        (bind _fade (Timeline|LaserFade PlayFromStart)
          (:Update
            (Rendering|Material|SetScalarParameterValue (Variables|Default|GetLaserMat) "Glow" (* _fade 1e+03) :!class /Script/Engine.MaterialInstanceDynamic))
          (:Finished
            (Development|SetHiddeninGame (Variables|Default|GetLaserPlane) true false)
            (Variables|Default|SetCanFire true))))
      (:then_1
        (if (and (Utilities|IsValid (Variables|/Game/Blueprints/BP_PlayerShip.BP_PlayerShip_C|GetWeaponsTarget (Variables|Default|GetPlayer))) (Variables|Default|GetCanSee))
          (Default|TakeDamage (Variables|/Game/Blueprints/BP_PlayerShip.BP_PlayerShip_C|GetWeaponsTarget (Variables|Default|GetPlayer)) (Variables|Default|GetDamage)))))))

(fn ConstructionScript
  (bind _returnvalue (Rendering|Material|CreateDynamicMaterialInstance "/Game/Materials/M_lightning.M_lightning" "None" :!class /Script/Engine.KismetMaterialLibrary))
  (bind _output_get (Variables|Default|SetLaserMat _returnvalue))
  (Rendering|Material|SetMaterial (Variables|Default|GetLaserPlane) 0 _output_get))