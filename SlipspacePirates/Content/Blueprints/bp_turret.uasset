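; Turret actor that aims its body at a target component or actor while active.
; A fast looping timer points the body from the guns toward the target, clamps relative pitch, then draws a debug visibility trace along the guns' forward vector.
; The trace result is unused.
; It also binds to the first BP_MusicManager's beat event, but that handler is empty.
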(event Custom|updateRotation
  (bind _fbx_turret_body (Variables|Default|GetFBX_Turret_Body))
  (bind _fbx_turret_guns (Variables|Default|GetFBX_Turret_Guns))
  (bind _returnvalue (Transformation|GetWorldLocation _fbx_turret_guns))
  (bind _relativerotation (Variables|/Script/Engine.SceneComponent|GetRelativeRotation _fbx_turret_body))
  (if (Variables|Default|GetActive)
    (Transformation|SetWorldRotation _fbx_turret_body (Math|Rotator|FindLookatRotation (Transformation|GetWorldLocation (Variables|Default|GetFBX_Turret_Guns)) (Transformation|GetWorldLocation (Variables|Default|GetTarget))) false false)
    (Transformation|SetRelativeRotation _fbx_turret_body (Math|Rotator|MakeRotator (.roll _relativerotation) (Math|Float|Clamp(Float) (.pitch _relativerotation) 0.0 1.8e+02) (.yaw _relativerotation)) false false)
    (Collision|LineTraceByChannel _returnvalue (+ _returnvalue (* (Math|Vector|GetForwardVector _fbx_turret_guns) 1.5e+04)) "TraceTypeQuery1" false 0 "ForDuration" true "(R=1.000000,G=0.000000,B=0.000000,A=1.000000)" "(R=0.000000,G=1.000000,B=0.000000,A=1.000000)" 0.01)))

(event Custom|OnBeatReciever)

(event EventBeginPlay
  (Utilities|Time|SetTimerbyEvent (delegate Custom|updateRotation) 0.01 true)
  (bind _outactors (Actor|GetAllActorsOfClass "/Game/Blueprints/BP_MusicManager.BP_MusicManager_C"))
  (EventDispatchers|BindEventtoOnBeat (Utilities|Array|Get(acopy) _outactors) (delegate Custom|OnBeatReciever)))

(fn ConstructionScript)