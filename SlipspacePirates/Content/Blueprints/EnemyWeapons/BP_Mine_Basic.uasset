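; BP_Mine_Basic is a basic enemy mine that drifts, spins and damages the player ship on contact.
; A timeline moves the mesh along its relative X axis while a looping timer applies roll.
; Sphere overlap with BP_PlayerShip subtracts directly from its Health variable, then calls Death.
; Taking any damage or outliving a short delay also calls Death, whose body is not defined here.
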(event OnComponentBeginOverlap(Sphere)
  (params (OverlappedComponent :type Primitive%20Component%20Object%20Reference) (OtherActor :type Actor%20Object%20Reference) (OtherComp :type Primitive%20Component%20Object%20Reference) (OtherBodyIndex :type Integer) (bFromSweep :type Boolean) (SweepResult :type Hit%20Result%20Structure%20%28by%20ref%29))
  (if (!= OtherActor self)
    (bind _asbp_player_ship (Utilities|Casting|CastToBP_PlayerShip OtherActor))
    (Variables|/Game/Blueprints/BP_PlayerShip.BP_PlayerShip_C|SetHealth _asbp_player_ship (- (Variables|/Game/Blueprints/BP_PlayerShip.BP_PlayerShip_C|GetHealth _asbp_player_ship) 0.05))
    (CallFunction|Death)))

(event Custom|Rotate
  (Transformation|AddRelativeRotation (Variables|Character|GetMesh) (Math|Rotator|MakeRotator (Variables|Default|GetRot) 0.0 0.0) false false))

(event EventBeginPlay
  (Utilities|Time|SetTimerbyEvent (delegate Custom|Rotate) 0.06 true)
  (Utilities|FlowControl|Sequence
    (:then_0
      (bind _driftup (Timeline|Drift PlayFromStart)
        (:Update
          (Transformation|SetRelativeLocation (Variables|Character|GetMesh) (Math|Vector|MakeVector (* _driftup 9e+02) 0.0 0.0) false false))))
    (:then_1
      (Utilities|FlowControl|Delay 4.5)
      (CallFunction|Death))))

(event EventTakeDamage
  (params (Damage :type Float%20%28single-precision%29))
  (CallFunction|Death))

(fn ConstructionScript)