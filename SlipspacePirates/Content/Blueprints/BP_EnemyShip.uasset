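; BP_EnemyShip is an enemy ship that moves its Cube endlessly along the spline of a slipspace tube.
; On BeginPlay it takes the first BP_SlipspaceTube found and starts a fast looping timer.
; Each timer call adds Speed to the travelled distance, wraps it by spline length, and sets the Cube's world location and rotation from the spline's local-space values, without sweep or delta-time scaling.
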(event Custom|Update
  (bind _cube (Variables|Default|GetCube))
  (bind _slipspacetrack (Variables|Default|GetSlipspaceTrack))
  (bind _spline (Variables|/Game/Blueprints/BP_SlipspaceTube.BP_SlipspaceTube_C|GetSpline _slipspacetrack))
  (bind _output_get (Variables|Default|SetTrackDist (+ (Variables|Default|GetTrackDist) (Variables|Default|GetSpeed))))
  (Transformation|SetWorldLocation _cube (Spline|GetLocationatDistanceAlongSpline _spline (Math|Float|%(Float) _output_get (Spline|GetSplineLength _spline)) "Local") false false)
  (Transformation|SetWorldRotation _cube (Spline|GetRotationatDistanceAlongSpline _spline (Math|Float|%(Float) _output_get (Spline|GetSplineLength _spline)) "Local") false false))

(event EventBeginPlay
  (bind _outactors (Actor|GetAllActorsOfClass "/Game/Blueprints/BP_SlipspaceTube.BP_SlipspaceTube_C"))
  (Variables|Default|SetSlipspaceTrack (Utilities|Array|Get(acopy) _outactors))
  (Utilities|Time|SetTimerbyEvent (delegate Custom|Update) 0.005 true))

(fn ConstructionScript)