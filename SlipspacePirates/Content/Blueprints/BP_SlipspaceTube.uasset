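; BP_SlipspaceTube is a spline-driven tube, named for slipspace, whose material receives the music tempo.
; The construction script adds a shadowless spline mesh at each spline point, shaped by that point's and the next's locations and tangents.
; Each mesh gets a dynamic slipspace material on its inner slot, with a BPS parameter computed from the first BP_MusicManager's BPM divided by 60.
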(event EventBeginPlay)

(fn ConstructionScript
  (bind _spline (Variables|Default|GetSpline))
  (for _index (range 0 (- (Spline|GetNumberOfSplinePoints (Variables|Default|GetSpline)) 1))
    (bind _returnvalue (AddComponent|AddSplineMeshComponent true))
    (bind _output_get (Variables|Default|SetSplineMesh _returnvalue))
    (Transformation|AttachComponentToComponent _output_get (Variables|Default|GetScene) "None" "KeepRelative" "KeepRelative" "KeepRelative" true)
    (SplineMesh|SetStartandEnd (Variables|Default|GetSplineMesh) (.Location (Spline|GetLocationandTangentatSplinePoint _spline _index "Local")) (.Tangent (Spline|GetLocationandTangentatSplinePoint _spline _index "Local")) (.Location (Spline|GetLocationandTangentatSplinePoint _spline (+ _index 1) "Local")) (.Tangent (Spline|GetLocationandTangentatSplinePoint _spline (+ _index 1) "Local")) true :!class /Script/Engine.SplineMeshComponent)
    (bind _returnvalue_2 (Rendering|Material|CreateDynamicMaterialInstance (Variables|Default|GetSlipspaceMaterial) "None" :!class /Script/Engine.KismetMaterialLibrary))
    (bind _output_get_2 (Variables|Default|SetSplineMat _returnvalue_2))
    (Rendering|Material|SetMaterialbyName (Variables|Default|GetSplineMesh) "M_InnerMat" _output_get_2)
    (bind _outactors (Actor|GetAllActorsOfClass "/Game/Blueprints/BP_MusicManager.BP_MusicManager_C"))
    (Rendering|Material|SetScalarParameterValue (Variables|Default|GetSplineMat) "BPS" (/ (Math|Conversions|ToFloat(Integer) (Variables|/Game/Blueprints/BP_MusicManager.BP_MusicManager_C|GetBPM (Utilities|Array|Get(acopy) _outactors))) 6e+01) :!class /Script/Engine.MaterialInstanceDynamic)
    (Rendering|SetCastShadow (Variables|Default|GetSplineMesh) false)))