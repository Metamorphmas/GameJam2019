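; Player turret that swings toward whatever lies under the mouse cursor and sets the hovered ShipComponent as the Player's highlighted WeaponsTarget.
; A fast looping timer, gated by Active, traces from the cursor while ignoring all turrets, falling back to the ray end on a miss.
; The body lerps toward that point with clamped pitch, and a debug trace shows the gun direction.
; It binds to BP_MusicManager's beat event, but the handler is empty.
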(event Custom|updateRotation
  (bind _returnvalue (Game|GetPlayerController 0))
  (bind _raycastdistance (Variables|Default|GetRayCastDistance))
  (bind _player (Variables|Default|GetPlayer))
  (bind _player_2 (Variables|Default|GetPlayer))
  (bind _fbx_turret_body (Variables|Default|GetFBX_Turret_Body))
  (bind _fbx_turret_body_2 (Variables|Default|GetFBX_Turret_Body))
  (bind _fbx_turret_guns (Variables|Default|GetFBX_Turret_Guns))
  (bind _fbx_turret_guns_2 (Variables|Default|GetFBX_Turret_Guns))
  (bind (_locationx _locationy) (Game|Player|GetMousePosition _returnvalue))
  (bind _returnvalue_2 (Transformation|GetWorldRotation _fbx_turret_guns))
  (bind _returnvalue_3 (Transformation|GetWorldLocation _fbx_turret_guns))
  (bind _returnvalue_4 (Transformation|GetWorldLocation _fbx_turret_guns_2))
  (bind _relativerotation (Variables|/Script/Engine.SceneComponent|GetRelativeRotation _fbx_turret_body))
  (bind _relativerotation_2 (Variables|/Script/Engine.SceneComponent|GetRelativeRotation _fbx_turret_body_2))
  (bind (_worldlocation _worlddirection) (Class|PlayerController|DeprojectScreenPositiontoWorld _returnvalue _locationx _locationy))
  (bind _returnvalue_5 (* _worlddirection _raycastdistance))
  (bind _returnvalue_6 (+ _worldlocation _returnvalue_5))
  (if (Variables|Default|GetActive)
    (bind (_outhit _returnvalue_7) (Collision|LineTraceForObjects _worldlocation _returnvalue_6 (Utilities|Array|MakeArray "ObjectTypeQuery2" "ObjectTypeQuery1") false (Variables|Default|GetcomponentsToIgnore) "None"))
    (if _returnvalue_7
      (Utilities|FlowControl|Sequence
        (:then_0
          (bind _output_get (Variables|Default|SetTargetRot (Math|Rotator|FindLookatRotation _returnvalue_3 (.Location (Collision|BreakHitResult _outhit)))))
          (Transformation|SetWorldRotation _fbx_turret_body (Math|Rotator|Lerp(Rotator) _returnvalue_2 _output_get 0.06 true) false false)
          (Transformation|SetRelativeRotation _fbx_turret_body (Math|Rotator|MakeRotator (.roll _relativerotation) (Math|Float|Clamp(Float) (.pitch _relativerotation) 0.0 1.8e+02) (.yaw _relativerotation)) false false)
          (Collision|LineTraceByChannel _returnvalue_4 (+ _returnvalue_4 (* (Math|Vector|GetForwardVector _fbx_turret_guns_2) (Variables|Default|GetRayCastDistance))) "TraceTypeQuery1" false 0 "ForDuration" true "(R=1.000000,G=0.000000,B=0.000000,A=1.000000)" "(R=0.000000,G=1.000000,B=0.000000,A=1.000000)" 0.01 :!label _label))
        (:then_1
          (bind _asship_component (Utilities|Casting|CastToShipComponent (.HitActor (Collision|BreakHitResult _outhit)))
            (:then
              (if (Utilities|IsValid (Variables|/Game/Blueprints/BP_PlayerShip.BP_PlayerShip_C|GetWeaponsTarget (Variables|Default|GetPlayer)))
                (if (not (== _asship_component (Variables|/Game/Blueprints/BP_PlayerShip.BP_PlayerShip_C|GetWeaponsTarget (Variables|Default|GetPlayer))))
                  (Default|Highlight (Variables|/Game/Blueprints/BP_PlayerShip.BP_PlayerShip_C|GetWeaponsTarget _player_2) false)
                  (bind _output_get_2 (Variables|/Game/Blueprints/BP_PlayerShip.BP_PlayerShip_C|SetWeaponsTarget _player_2 _asship_component :!label _label_2))
                  (Default|Highlight _output_get_2 true))
                (else
                  (goto _label_2))))
            (:CastFailed
              (if (Utilities|IsValid (Variables|/Game/Blueprints/BP_PlayerShip.BP_PlayerShip_C|GetWeaponsTarget _player)) :!label _label_3
                (Default|Highlight (Variables|/Game/Blueprints/BP_PlayerShip.BP_PlayerShip_C|GetWeaponsTarget _player) false)
                (Variables|/Game/Blueprints/BP_PlayerShip.BP_PlayerShip_C|SetWeaponsTarget _player 0))))))
      (else
        (Utilities|FlowControl|Sequence
          (:then_0
            (bind _output_get_3 (Variables|Default|SetTargetRot (Math|Rotator|FindLookatRotation _returnvalue_3 _returnvalue_6)))
            (Transformation|SetWorldRotation _fbx_turret_body_2 (Math|Rotator|Lerp(Rotator) _returnvalue_2 _output_get_3 0.06 true) false false)
            (Transformation|SetRelativeRotation _fbx_turret_body_2 (Math|Rotator|MakeRotator (.roll _relativerotation_2) (Math|Float|Clamp(Float) (.pitch _relativerotation_2) 0.0 1.8e+02) (.yaw _relativerotation_2)) false false)
            (goto _label))
          (:then_1
            (goto _label_3)))))))

(event Custom|OnBeatReciever
  (params (BeatCount :type Integer) (MusicTime :type Float%20%28single-precision%29)))

(event EventBeginPlay
  (Utilities|Time|SetTimerbyEvent (delegate Custom|updateRotation) 0.005 true)
  (bind _outactors (Actor|GetAllActorsOfClass "/Game/Blueprints/BP_MusicManager.BP_MusicManager_C"))
  (EventDispatchers|BindEventtoOnBeat (Utilities|Array|Get(acopy) _outactors) (delegate Custom|OnBeatReciever))
  (bind _outactors_2 (Actor|GetAllActorsOfClass "BP_PlayerTurret_C"))
  (Variables|Default|SetcomponentsToIgnore _outactors_2))

(fn ConstructionScript)