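; BP_EnemyTest is a test enemy that loops along a slipspace tube spline while carrying two turrets aimed at the player ship.
; On BeginPlay it finds the first BP_SlipspaceTube and sets both child-actor turrets' targets to the player ship's mesh.
; Each tick advances a fixed distance without delta-time scaling, wraps by spline length, and applies the spline's local-space transform to the Cube as world location and rotation.
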(event EventBeginPlay
  (bind _outactors (Actor|GetAllActorsOfClass "/Game/Blueprints/BP_SlipspaceTube.BP_SlipspaceTube_C"))
  (Variables|Default|SetSlipspaceTrack (Utilities|Array|Get(acopy) _outactors))
  (bind _asbp_turret (Utilities|Casting|CastToBP_Turret (Variables|/Script/Engine.ChildActorComponent|GetChildActor (Variables|Default|Getbp_turret))))
  (bind _asbp_turret_2 (Utilities|Casting|CastToBP_Turret (Variables|/Script/Engine.ChildActorComponent|GetChildActor (Variables|Default|GetChildActor))))
  (bind _asbp_player_ship (Utilities|Casting|CastToBP_PlayerShip (Game|Player|GetPlayerPawn 0)))
  (Variables|/Game/Blueprints/bp_turret.BP_Turret_C|SetTarget _asbp_turret (Variables|/Game/Blueprints/BP_PlayerShip.BP_PlayerShip_C|GetStaticMesh _asbp_player_ship))
  (Variables|/Game/Blueprints/bp_turret.BP_Turret_C|SetTarget _asbp_turret_2 (Variables|/Game/Blueprints/BP_PlayerShip.BP_PlayerShip_C|GetStaticMesh _asbp_player_ship)))

(event EventTick
  (params (DeltaSeconds :type Float%20%28single-precision%29))
  (bind _cube (Variables|Default|GetCube))
  (bind _slipspacetrack (Variables|Default|GetSlipspaceTrack))
  (bind _spline (Variables|/Game/Blueprints/BP_SlipspaceTube.BP_SlipspaceTube_C|GetSpline _slipspacetrack))
  (bind _output_get (Variables|Default|SetTrackDist (+ (Variables|Default|GetTrackDist) 1.2e+02)))
  (Transformation|SetWorldLocation _cube (Spline|GetLocationatDistanceAlongSpline _spline (Math|Float|%(Float) _output_get (Spline|GetSplineLength _spline)) "Local") false false)
  (Transformation|SetWorldRotation _cube (Spline|GetRotationatDistanceAlongSpline _spline (Math|Float|%(Float) _output_get (Spline|GetSplineLength _spline)) "Local") false false))

(fn ConstructionScript)