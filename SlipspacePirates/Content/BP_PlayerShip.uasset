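; Player ship for a rhythm-driven flight game, gaining speed when AddThrust is pressed on the music's beat.
; A fast looping timer moves ShipCenter forward, rolls it by strafe velocity and eases the mesh's offset toward a wheel-set hover distance, swinging it around the center.
; BP_MusicManager grades each press to boost or cut velocity; successful hits delay a gradual slowdown.
; The thrust axis only responds to negative input, and ChangeCamera toggles cockpit view.
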(event Custom|Init
  (bind _outactors (Actor|GetAllActorsOfClass "/Game/BP_MusicManager.BP_MusicManager_C"))
  (Variables|Default|SetMusicManager (Utilities|Array|Get(acopy) _outactors))
  (Utilities|Time|SetTimerbyEvent (delegate Custom|Update) 0.005 true)
  (Variables|/Script/Engine.PlayerController|SetbShowMouseCursor (Game|GetPlayerController 0) true))

(event Custom|Update
  (bind _shipcenter (Variables|Default|GetshipCenter))
  (bind _shipcenter_2 (Variables|Default|GetshipCenter))
  (bind _relativerotation (Variables|/Script/Engine.SceneComponent|GetRelativeRotation _shipcenter_2))
  (Utilities|FlowControl|Sequence
    (:then_0
      (Transformation|SetWorldLocation _shipcenter (+ (Transformation|GetWorldLocation _shipcenter) (* (Transformation|GetActorForwardVector) (Variables|Default|GetVelocity))) false false)
      (Transformation|SetRelativeRotation _shipcenter_2 (Math|Rotator|MakeRotator (Math|Float|Lerp (.roll _relativerotation) (+ (Variables|Default|GetstrafeVelocity) (.roll _relativerotation)) 0.1) 0.0 0.0) false false)
      (bind _output_get (Variables|Default|SethoverDist (Math|Float|Lerp (Variables|Default|GethoverDist) (Variables|Default|GettargetHoverDist) 0.005)))
      (Transformation|SetRelativeLocation (Variables|Default|GetStaticMesh) (Math|Vector|MakeVector 0.0 0.0 _output_get) false false))
    (:then_1
      (if (Variables|Default|GetisSlowingDown)
        (Variables|Default|SetVelocity (Math|Float|Lerp (Variables|Default|GetVelocity) 0.0 0.001))))))

(event Custom|StartSlowingDown
  (Variables|Default|SetisSlowingDown true)
  (Development|PrintString "SlowingDown!"))

(event EventBeginPlay
  (CallFunction|Init))

(event Input|ActionEvents|InputActionChangeCamera
  (params (Key :type Key%20Structure))
  (bind _cockpitcamera (Variables|Default|GetCockpitCamera))
  (bind _maincamera (Variables|Default|GetMainCamera))
  (:Pressed
    (if (Variables|Default|GetisFirstPerson)
      (Components|Activation|SetActive _maincamera true false)
      (Components|Activation|SetActive _cockpitcamera false false)
      (Variables|Default|SetisFirstPerson false)
      (else
        (Components|Activation|SetActive _maincamera false false)
        (Components|Activation|SetActive _cockpitcamera true false)
        (Variables|Default|SetisFirstPerson true)))))

(event Input|ActionEvents|InputActionAddThrust
  (params (Key :type Key%20Structure))
  (bind _maxlinearvelocity (Variables|Default|GetMaxLinearVelocity))
  (:Pressed
    (bind _closeness (Default|GetonBeatCloseness (Variables|Default|GetMusicManager)))
    (Development|PrintString (Utilities|String|EnumtoString _closeness) true true "(R=0.045387,G=1.000000,B=0.000000,A=1.000000)" 0.1)
    (switch Utilities|FlowControl|Switch|SwitchonOnBeat _closeness
      (:NewEnumerator0
        (Variables|Default|SetVelocity (Math|Float|Clamp(Float) (+ (Variables|Default|GetVelocity) 5.0) 0.0 _maxlinearvelocity) :!label _label)
        (Utilities|Time|SetTimerbyEvent (delegate Custom|StartSlowingDown) (Variables|Default|GetSlowdownCooldown) :!label _label_2)
        (Variables|Default|SetisSlowingDown false))
      (:NewEnumerator1
        (goto _label))
      (:NewEnumerator2
        (Variables|Default|SetVelocity (Math|Float|Clamp(Float) (+ (Variables|Default|GetVelocity) 2.0) 0.0 _maxlinearvelocity))
        (goto _label_2))
      (:NewEnumerator3
        (Variables|Default|SetVelocity (Math|Float|Clamp(Float) (+ (Variables|Default|GetVelocity) -2.0) 0.0 _maxlinearvelocity))))))

(event Input|AxisEvents|InputAxisWheelDist
  (params (AxisValue :type Float%20%28single-precision%29))
  (if (!= AxisValue 0.0)
    (Variables|Default|SettargetHoverDist (Math|Float|Clamp(Float) (+ (Variables|Default|GettargetHoverDist) (* AxisValue 5e+01)) -1e+03 -4e+02))))

(event Input|AxisEvents|InputAxisThrust
  (params (AxisValue :type Float%20%28single-precision%29))
  (if (< AxisValue 0.0)
    (Variables|Default|SetVelocity (Math|Float|Clamp(Float) (+ (Variables|Default|GetVelocity) (* (Variables|Default|GetAcceleration) AxisValue)) 0.0 (Variables|Default|GetMaxLinearVelocity)))))

(event Input|AxisEvents|InputAxisStrafe
  (params (AxisValue :type Float%20%28single-precision%29))
  (bind _maxstrafevelocity (Variables|Default|GetMaxStrafeVelocity))
  (if (!= AxisValue 0.0)
    (Variables|Default|SetstrafeVelocity (Math|Float|Clamp(Float) (+ (Variables|Default|GetstrafeVelocity) (* (Variables|Default|GetStrafeAcceleration) AxisValue)) (* _maxstrafevelocity -1.0) _maxstrafevelocity))
    (else
      (Variables|Default|SetstrafeVelocity (Math|Float|Lerp (Variables|Default|GetstrafeVelocity) 0.0 0.003)))))

(fn ConstructionScript)